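; BP_minsec is a debug timer Blueprint that prints elapsed time as minutes and seconds on screen.
; Tick accumulates delta time into a Seconds variable, then derives minutes by dividing by 60 and seconds by modulo 60, truncating both.
; The values are joined with Russian unit labels and reprinted every frame with a very short duration, so the text reads as a live counter.
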(event EventTick
  (params (DeltaSeconds :type Float%20%28single-precision%29))
  (bind _output_get (Variables|Default|SetSeconds (+ DeltaSeconds (Variables|Default|GetSeconds))))
  (Development|PrintString (Utilities|String|Append (Utilities|String|ToString(Integer) (Math|Float|Truncate (/ (+ DeltaSeconds (Variables|Default|GetSeconds)) 6e+01))) "  минут,   " (Utilities|String|ToString(Integer) (Math|Float|Truncate (Math|Float|%(Float) _output_get 6e+01))) " секунд.") true true "(R=0.000000,G=0.660000,B=1.000000,A=1.000000)" 0.005))

(fn ConstructionScript)