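; BP_metronom is a test actor that acts as a metronome, printing alternating on-screen greeting and farewell messages in Russian.
; BeginPlay starts a looping five-second timer whose event drives a FlipFlop between the red "Привет!!!" and green "Пока!!!" prints.
; Tick is empty, and a disconnected DeltaSeconds accumulator with modulo and branch nodes remains in the graph but never runs.
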(event Custom|Timer
  (Utilities|FlowControl|FlipFlop
    (:A
      (Development|PrintString "Привет!!!" true true "(R=1.000000,G=0.000000,B=0.069038,A=1.000000)" 1.0))
    (:B
      (Development|PrintString "Пока!!!" true true "(R=0.000000,G=1.000000,B=0.109613,A=1.000000)" 1.0))))

(event EventBeginPlay
  (Utilities|Time|SetTimerbyEvent (delegate Custom|Timer) 5.0 true))

(event EventTick
  (params (DeltaSeconds :type Float%20%28single-precision%29)))

(fn ConstructionScript)