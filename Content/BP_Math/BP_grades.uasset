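; BP_grades is a math exercise Blueprint that prints a Russian rating for its Grade variable when another actor overlaps it.
; On ActorBeginOverlap, a chain of nested range checks tests Grade against five bands from highest to lowest and prints the matching message, from excellent praise down to "bad".
; Grades outside the 1 to 100 scale print nothing, and the construction script is empty.
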(event Collision|EventActorBeginOverlap
  (params (OtherActor :type Actor%20Object%20Reference))
  (bind _grade (Variables|Default|GetGrade))
  (bind _grade_2 (Variables|Default|GetGrade))
  (bind _grade_3 (Variables|Default|GetGrade))
  (bind _grade_4 (Variables|Default|GetGrade))
  (bind _grade_5 (Variables|Default|GetGrade))
  (if (and (>= _grade_2 81) (<= _grade_2 100))
    (Development|PrintString "Лучше некуда!!! Проверяем гитхаб!")
    (elif (and (>= _grade_3 61) (<= _grade_3 80))
      (Development|PrintString "Отлично")
      (elif (and (>= _grade_4 41) (<= _grade_4 60))
        (Development|PrintString "Хорошо")
        (elif (and (>= _grade_5 21) (<= _grade_5 40))
          (Development|PrintString "Удовлетворительно")
          (elif (and (>= _grade 1) (<= _grade 20))
            (Development|PrintString "Плохо")))))))

(fn ConstructionScript)